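; Floor tile for an endless runner that requests the next tile from EndlessRunnerGameMode when the RunCharacter overlaps its SpawnTrigger, then destroys itself after a delay unless the runner is dead.
; A DeathTrigger overlap kills the runner.
; The construction script randomly adds either an obstacle or a pickup as a child actor at one of five spawn points.
; GetAttachPointTransform exposes the AttachPoint's world transform.
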(event `self.Spawn Trigger.OnComponentBeginOverlap`
  (params (OtherActor :type "Actor Object Reference") (OtherComp :type "PrimitiveComponent Object Reference") (OtherBodyIndex :type Integer) (bFromSweep :type Boolean) (SweepResult :type "HitResult Structure (by ref)"))
  (bind _asrun_character (cast `/Game/Blueprints/Characters/RunCharacter` OtherActor))
  (bind _asendless_runner_game_mode (cast `/Game/Blueprints/GameModes/EndlessRunnerGameMode` (`GameplayStatics.GetGameMode`)))
  (`/Game/Blueprints/GameModes/EndlessRunnerGameMode.AddTile` _asendless_runner_game_mode)
  (if (not (`/Game/Blueprints/Characters/RunCharacter.Is Dead` _asrun_character))
    (`KismetSystemLibrary.Delay` 3.0)
    (`self.K2_DestroyActor`)))

(event `self.Death Trigger.OnComponentBeginOverlap`
  (params (OtherActor :type "Actor Object Reference") (OtherComp :type "PrimitiveComponent Object Reference") (OtherBodyIndex :type Integer) (bFromSweep :type Boolean) (SweepResult :type "HitResult Structure (by ref)"))
  (bind _asrun_character (cast `/Game/Blueprints/Characters/RunCharacter` OtherActor))
  (`/Game/Blueprints/Characters/RunCharacter.Die` _asrun_character))

(fn `GetAttachPointTransform`
  (returns (`Attach Point Transform` :type "Transform Structure"))
  (return (`SceneComponent.K2_GetComponentToWorld` (`self.AttachPoint`))))

(fn `SetSpawnPoints`
  (set `self.SpawnPoints` (`|MakeArray` (`SceneComponent.GetRelativeTransform` (`self.Spawn Point 1`)) (`SceneComponent.GetRelativeTransform` (`self.Spawn Point 2`)) (`SceneComponent.GetRelativeTransform` (`self.Spawn Point 3`)) (`SceneComponent.GetRelativeTransform` (`self.Spawn Point 4`)) (`SceneComponent.GetRelativeTransform` (`self.Spawn Point 5`)))))

(fn `SpawnObstacle`
  (bind _spawnpoints (`self.SpawnPoints`))
  (bind _obstacles (`self.Obstacles`))
  (bind _returnvalue (`AddComponent|ChildActorComponent_2627` :`RelativeTransform` (`KismetArrayLibrary.Array_Get` _spawnpoints (`KismetMathLibrary.RandomIntegerInRange` 0 (`KismetArrayLibrary.Array_LastIndex` _spawnpoints)))))
  (`ChildActorComponent.SetChildActorClass` _returnvalue (`KismetArrayLibrary.Array_Get` _obstacles (`KismetMathLibrary.RandomIntegerInRange` 0 (`KismetArrayLibrary.Array_LastIndex` _obstacles)))))

(fn `SpawnPickup`
  (bind _spawnpoints (`self.SpawnPoints`))
  (bind _pickups (`self.Pickups`))
  (bind _returnvalue (`AddComponent|ChildActorComponent_2664` :`RelativeTransform` (`KismetArrayLibrary.Array_Get` _spawnpoints (`KismetMathLibrary.RandomIntegerInRange` 0 (`KismetArrayLibrary.Array_LastIndex` _spawnpoints)))))
  (`ChildActorComponent.SetChildActorClass` _returnvalue (`KismetArrayLibrary.Array_Get` _pickups (`KismetMathLibrary.RandomIntegerInRange` 0 (`KismetArrayLibrary.Array_LastIndex` _pickups)))))

(fn `UserConstructionScript`
  (`self.SetSpawnPoints`)
  (switch `int` (`KismetMathLibrary.RandomIntegerInRange` 0 1)
    (:`Default`
      (`self.SpawnObstacle` :!label _label))
    (:`0`
      (goto _label))
    (:`1`
      (`self.SpawnPickup`))))