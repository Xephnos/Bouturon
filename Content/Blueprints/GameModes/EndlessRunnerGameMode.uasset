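; Game mode for an endless runner that creates the HUD and lays the initial stretch of track at play start.
; AddTile spawns a random tile class at the next spawn point, then moves that point to the new tile's attach transform to chain pieces end to end.
; A counter diverts AddTile to spawn a random ramp once it exceeds a threshold, which is re-randomized after each ramp.
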(event `self.ReceiveBeginPlay`
  (bind _returnvalue (`|CreateWidget` "/Game/Blueprints/UMG/EndllessRunnerHUD.EndllessRunnerHUD_C"))
  (`UserWidget.AddToViewport` _returnvalue 0)
  (for _ (range 1 21)
    (`self.AddTile`)))

(fn `AddRamp`
  (bind _ramps (`self.Ramps`))
  (bind _returnvalue (`|SpawnActorFromClass` (`KismetArrayLibrary.Array_Get` _ramps (`KismetMathLibrary.RandomIntegerInRange` 0 (`KismetArrayLibrary.Array_LastIndex` _ramps))) (`self.Next Spawn Point`) "Undefined" "OverrideRootScale"))
  (bind _astile_basic (cast `/Game/Blueprints/Tiles/Tile_Basic` _returnvalue))
  (bind _attach_point_transform (`/Game/Blueprints/Tiles/Tile_Basic.GetAttachPointTransform` _astile_basic))
  (set `self.Next Spawn Point` _attach_point_transform)
  (set `self.Ramp Counter` 0)
  (set `self.Random Ramp Spawn` (`KismetMathLibrary.RandomIntegerInRange` 5 10)))

(fn `AddTile`
  (bind _tiles (`self.Tiles`))
  (if (> (`self.Ramp Counter`) (`self.Random Ramp Spawn`))
    (`self.AddRamp`)
    (else
      (bind _returnvalue (`|SpawnActorFromClass` (`KismetArrayLibrary.Array_Get` _tiles (`KismetMathLibrary.RandomIntegerInRange` 0 (`KismetArrayLibrary.Array_LastIndex` _tiles))) (`self.Next Spawn Point`) "Undefined" "OverrideRootScale"))
      (bind _astile_basic (cast `/Game/Blueprints/Tiles/Tile_Basic` _returnvalue))
      (bind _attach_point_transform (`/Game/Blueprints/Tiles/Tile_Basic.GetAttachPointTransform` _astile_basic))
      (set `self.Next Spawn Point` _attach_point_transform)
      (set `self.Ramp Counter` (+ (`self.Ramp Counter`) 1)))))

(fn `UserConstructionScript`)